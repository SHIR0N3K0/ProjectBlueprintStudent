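; BP_Door is an interactable double door that can optionally require a key to open.
; On BeginPlay it caches the BP_Key actor returned by GetActorOfClass.
; The Interactible event toggles through a FlipFlop when Condition is false, or when the key's Key1Gotten flag is set.
; The FlipFlop plays or reverses a Timeline that yaws the two meshes in opposite directions, scaled by AngleRotation.
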(event `self.ReceiveBeginPlay`
  (bind _returnvalue (`GameplayStatics.GetActorOfClass` "/Game/Blueprints/BP_Key.BP_Key_C"))
  (set `self.NewVar` _returnvalue))

(event `/Game/Blueprints/BPI_Interact.Interactible`
  (if (not (`self.Condition`))
    (`/Engine/EditorBlueprintResources/StandardMacros.FlipFlop` :!label _label
      (:`A`
        (bind (_direction _newtrack_0) (`Timeline|Timeline` :!label _label_2)
          (:`Update`
            (bind _returnvalue (* _newtrack_0 (`self.AngleRotation`)))
            (`SceneComponent.K2_SetRelativeRotation` (`self.StaticMesh`) (`KismetMathLibrary.MakeRotator` 0.0 0.0 _returnvalue) false false)
            (`SceneComponent.K2_SetRelativeRotation` (`self.StaticMesh1`) (`KismetMathLibrary.MakeRotator` 0.0 0.0 (* _returnvalue -1.0)) false false))))
      (:`B`
        (goto _label_2 :!via `Reverse`)))
    (elif (`/Game/Blueprints/BP_Key.Key 1 gotten` (`self.NewVar`))
      (goto _label))))

(fn `UserConstructionScript`)
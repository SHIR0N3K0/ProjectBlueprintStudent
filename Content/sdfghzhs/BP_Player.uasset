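; BP_Player is a player Character that handles Enhanced Input actions for move, jump and look.
; IA_Move fires only on Started, adding fixed full-scale forward and right input relative to control yaw, without reading the action value.
; IA_Jump starts a jump and stops it on Canceled.
; IA_Look passes zero to pitch and yaw, so it does not turn the view.
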(event `EnhancedInput|/Game/sdfghzhs/Input/IA_Move`
  (params (ActionValue :type Boolean) (ElapsedSeconds :type "Float (double-precision)") (TriggeredSeconds :type "Float (double-precision)") (InputAction :type "InputAction Object Reference" :default "/Game/sdfghzhs/Input/IA_Move.IA_Move"))
  (bind (_returnvalue_roll _returnvalue_pitch _returnvalue_yaw) (`KismetMathLibrary.BreakRotator` (`self.GetControlRotation`)))
  (:`Started`
    (`self.AddMovementInput` (`KismetMathLibrary.GetForwardVector` (`KismetMathLibrary.MakeRotator` 0.0 0.0 _returnvalue_yaw)))
    (`self.AddMovementInput` (`KismetMathLibrary.GetRightVector` (`KismetMathLibrary.MakeRotator` 0.0 0.0 _returnvalue_yaw)))))

(event `EnhancedInput|/Game/sdfghzhs/Input/IA_Jump`
  (params (ActionValue :type Boolean) (ElapsedSeconds :type "Float (double-precision)") (TriggeredSeconds :type "Float (double-precision)") (InputAction :type "InputAction Object Reference" :default "/Game/sdfghzhs/Input/IA_Jump.IA_Jump"))
  (:`Started`
    (`self.Jump`))
  (:`Canceled`
    (`self.StopJumping`)))

(event `EnhancedInput|/Game/sdfghzhs/Input/IA_Look`
  (params (ActionValue :type Boolean) (ElapsedSeconds :type "Float (double-precision)") (TriggeredSeconds :type "Float (double-precision)") (InputAction :type "InputAction Object Reference" :default "/Game/sdfghzhs/Input/IA_Look.IA_Look"))
  (:`Triggered`
    (`self.AddControllerPitchInput` 0.0)
    (`self.AddControllerYawInput` 0.0)))

(fn `UserConstructionScript`)